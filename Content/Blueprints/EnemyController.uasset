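; EnemyController is an early Blueprint for enemy attack selection, with only an Attack function implemented.
; Attack appends a random integer below 99 to the AttackedAlready array, then loops over it.
; The loop compares each element with itself and both branches return a fresh random integer, so it exits on the first element without filtering repeats.
; The event graph and construction script are empty.
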(fn `Attack`
  (returns (OutAttack :type Integer))
  (bind _returnvalue (`KismetMathLibrary.RandomInteger` 99))
  (bind _attacked_already (`self.Attacked Already`))
  (`KismetArrayLibrary.Array_Set` _attacked_already (`KismetArrayLibrary.Array_Length` _attacked_already) _returnvalue true)
  (for (_array_element _array_index) _attacked_already
    (if (== (`|GetArrayItem` _attacked_already _array_index) _array_element)
      (return (`KismetMathLibrary.RandomInteger` 99))
      (else
        (return _returnvalue)))))

(fn `UserConstructionScript`)