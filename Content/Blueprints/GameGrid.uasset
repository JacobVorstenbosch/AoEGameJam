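; GameGrid is a grid actor that tracks enemy and player tank positions and handles explosions on a grid cell.
; Explode takes a cell index, looks up its location in GridArray, and spawns an explosion particle effect and sound there.
; It then scans the parallel location and reference arrays for both sides and destroys every tank on that cell, leaving the arrays unmodified.
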(event `self.ReceiveBeginPlay`)

(fn `Explode`
  (params (InCoord :type Integer))
  (bind _output (`|GetArrayItem` (`self.GridArray`) InCoord))
  (`GameplayStatics.SpawnEmitterAtLocation` "/Game/StarterContent/Particles/P_Explosion.P_Explosion" _output)
  (`GameplayStatics.PlaySoundAtLocation` "/Game/Audio/sfx/sfx_boat-explosion.sfx_boat-explosion" _output (struct) 1.0 1.0 0.0 null null null)
  (for (_array_element _array_index) (`self.EnemyLocations`)
    (if (== _array_element InCoord)
      (`self.K2_DestroyActor` (`|GetArrayItem` (`self.EnemyTankRefs`) _array_index))))
  (for (_array_element_2 _array_index_2) (`self.PlayerLocations`)
    (if (== _array_element_2 InCoord)
      (`self.K2_DestroyActor` (`|GetArrayItem` (`self.PlayerTankRefs`) _array_index_2)))))

(fn `UserConstructionScript`)